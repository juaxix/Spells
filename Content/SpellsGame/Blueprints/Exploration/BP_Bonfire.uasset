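; BP_Bonfire is an interactable bonfire that acts as a save point.
; Interacting sets FireActive, writes the save game through SpellsGameModeBase, prints a confirmation and activates the fire particle system.
; When its state is restored from a save, it reactivates the particles if FireActive is set, so lit bonfires stay lit.
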(event EventOnRestoredStatefromSaveGame
  (if (Variables|Default|GetbFireActive)
    (Components|Activation|Activate (Variables|Default|GetParticleSystem) false)))

(event EventInteract
  (params (InstigatorPawn :type Pawn%20Object%20Reference))
  (bind _asspells_game_mode_base (Utilities|Casting|CastToSpellsGameModeBase (Game|GetGameMode)))
  (Variables|Default|SetbFireActive true)
  (Class|SpellsGameModeBase|WriteSaveGame _asspells_game_mode_base)
  (Development|PrintString "WORLD SAVED")
  (Components|Activation|Activate (Variables|Default|GetParticleSystem) false))

(fn ConstructionScript)