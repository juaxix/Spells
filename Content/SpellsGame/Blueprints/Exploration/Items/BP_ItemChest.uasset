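; BP_ItemChest is an interactable chest that opens only for a pawn holding the required key card tag and grants credits.
; Interact removes the tag from the pawn's SActionsComponent active tags and plays a timeline that rotates the lid open.
; On first opening it grants credits through SPlayerState, zeroes them, then fires particles and hides the gold.
; Interacting while open reverses the lid; a missing key prints the required tag.
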(event EventInteract
  (params (InstigatorPawn :type Pawn%20Object%20Reference))
  (bind _returnvalue (Actor|GetComponentbyClass InstigatorPawn "/Script/Spells.SActionsComponent"))
  (bind _activegameplaytags (Variables|/Script/Spells.SActionsComponent|GetActiveGameplayTags _returnvalue))
  (Utilities|IsValid InstigatorPawn
    (:Is%20Valid
      (if (Variables|Default|GetbOpened)
        (Utilities|FlowControl|Sequence
          (:then_0
            (bind _rotationfactor (Timeline|Open%20Chest Reverse)
              (:Update
                (Transformation|SetRelativeRotation (Variables|Default|GetLidStaticMesh) (Math|Rotator|MakeRotator 0.0 (* _rotationfactor (Variables|Default|GetOpenedAngle)) 0.0) false false))))
          (:then_1
            (Variables|Default|SetbOpened false)))
        (elif (GameplayTags|HasTag _activegameplaytags (Variables|Default|GetRequiredKeyCardTag) true)
          (GameplayTags|RemoveGameplayTag _activegameplaytags (Variables|Default|GetRequiredKeyCardTag) :!class /Script/GameplayTags.BlueprintGameplayTagLibrary)
          (Utilities|FlowControl|Sequence
            (:then_0
              (Variables|Default|SetbOpened true)
              (Timeline|Open%20Chest Play))
            (:then_1
              (if (> (Variables|Default|GetCreditsGranted) 0)
                (Utilities|IsValid InstigatorPawn
                  (:Is%20Valid
                    (bind _assplayer_state (Utilities|Casting|CastToSPlayerState (Variables|/Script/Engine.Pawn|GetPlayerState InstigatorPawn)))
                    (Class|SPlayerState|GrantCredits _assplayer_state (Variables|Default|GetCreditsGranted))
                    (Variables|Default|SetCreditsGranted 0)
                    (Utilities|FlowControl|Delay 0.2)
                    (Components|Activation|Activate (Variables|Default|GetParticleSystem) true)
                    (Development|SetHiddeninGame (Variables|Default|GetGold) true false))))))
          (else
            (Development|PrintString (GameplayTags|GetDebugStringfromGameplayTag (Variables|Default|GetRequiredKeyCardTag)) true true "(R=1.000000,G=0.195844,B=0.037901,A=1.000000)")))))))

(fn ConstructionScript)