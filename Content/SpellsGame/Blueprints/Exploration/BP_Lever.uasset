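; Networked exploration lever that toggles its handle via a timeline, then grants the instigator a key card gameplay tag and triggers a linked actor's interaction.
; Registers with Photon Cloud under a hashed display name and sends the instigator ID on interaction so other clients replay it.
; Lever state is stored in a custom room property, initialized by the master and read by other clients at BeginPlay to catch up.
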(event Custom|DO%20Interaction
  (params (Instigator%20Pawn :type Pawn%20Object%20Reference))
  (bind _returnvalue (Actor|GetComponentbyClass Instigator%20Pawn "/Script/Spells.SActionsComponent"))
  (bind _handlermesh (Variables|Default|GetHandlerMesh))
  (bind _levelerangle (Variables|Default|GetLevelerAngle))
  (bind _relativerotation (Variables|/Script/Engine.SceneComponent|GetRelativeRotation _handlermesh))
  ;[0.9823 0.7304 0] Cosmetics + Gameplay
  (Utilities|FlowControl|FlipFlop
    (:A
      (bind (_direction _anglealpha) (Timeline|HandlerRotation PlayFromStart)
        (:Update
          (Transformation|SetRelativeRotation _handlermesh (Math|Rotator|MakeRotator (.roll _relativerotation) (Math|Float|Lerp (.pitch _relativerotation) (Utilities|Select :Index _direction :Forward _levelerangle :Backward (* _levelerangle -1.0)) _anglealpha) (.yaw _relativerotation)) false false))
        (:Finished
          ;[0.4565 0.8361 1] Gameplay - Give key
          (Utilities|IsValid Instigator%20Pawn
            (:Is%20Valid
              (Utilities|IsValid _returnvalue
                (:Is%20Valid
                  (GameplayTags|AddGameplayTag (Variables|/Script/Spells.SActionsComponent|GetActiveGameplayTags _returnvalue) (Variables|Default|GetKeyCardTag) :!class /Script/GameplayTags.BlueprintGameplayTagLibrary))
                (:Is%20Not%20Valid
                  _)))
            (:Is%20Not%20Valid
              _))
          ;;[1 1 1] interact with linked actor - chain
          (bind _selectedactor (Variables|Default|GetSelectedActor)
            (:then
              (Class|SInteractableInterface|Interact(Message) _selectedactor Instigator%20Pawn))
            (:else)))))
    (:B
      (Timeline|HandlerRotation ReverseFromEnd))))

(event Custom|Replicate%20Interacted
  (params (NewInteracted :type Boolean))
  ;[1 0 0] Replicate bool
  (bind _output_get (Variables|Default|SetbInteracted NewInteracted))
  (bind _returnvalue (Class|PhotonJSON|SetBoolean (Class|PhotonJSON|Create self) (Variables|PhotonCloud|GetLeverInteractionReplicationKey) _output_get))
  (Class|PhotonCloudObject|AddCustomRoomProperties (Variables|PhotonCloud|GetPhoton%20Cloud%20BP%20Ref) _returnvalue))

(event EventBeginPlay
  (bind _returnvalue (Subsystems|GetPhotonCloudSubsystem))
  (bind _cachedhashedname (Variables|PhotonCloud|GetCachedHashedName))
  (bind _returnvalue_2 (Class|PhotonCloudSubsystem|GetPhotonCloudAPI _returnvalue))
  ;[1 0.574 0.9164] Begin play - cache , bind, set/get room prop
  ;;[1 1 1] cache photon
  (bind _asbp_photon_cloud_object (Utilities|Casting|CastToBP_PhotonCloudObject _returnvalue_2))
  (bind _output_get (Variables|PhotonCloud|SetPhoton%20Cloud%20BP%20Ref _asbp_photon_cloud_object))
  (if (Utilities|Enum|Equal(Enum) (Class|PhotonCloudObject|GetState _returnvalue_2) "JOINED")
    (Class|PhotonCloudObject|RegisterObservedMechanicsActor _output_get _cachedhashedname self)
    (Variables|PhotonCloud|SetLeverInteractionReplicationKey (Utilities|String|Append "lev_" (Utilities|String|ToString(Byte) (Math|Conversions|ToByte(Integer) _cachedhashedname))))
    (if (Class|PhotonCloudObject|AmIMaster (Variables|PhotonCloud|GetPhoton%20Cloud%20BP%20Ref))
      ;;[1 1 1] first replication
      (CallFunction|ReplicateInteracted (Variables|Default|GetbInteracted))
      (else
        ;;[1 1 1] set rotation if alreaded interacted
        (if (Class|PhotonJSON|Contains (Class|PhotonCloudObject|GetCustomRoomProperties (Variables|PhotonCloud|GetPhoton%20Cloud%20BP%20Ref)) (Variables|PhotonCloud|GetLeverInteractionReplicationKey))
          (if (Math|Boolean|NotEqual(Boolean) (Variables|Default|GetbInteracted) (Class|PhotonJSON|GetBoolean (Class|PhotonCloudObject|GetCustomRoomProperties (Variables|PhotonCloud|GetPhoton%20Cloud%20BP%20Ref)) (Variables|PhotonCloud|GetLeverInteractionReplicationKey)))
            (Variables|Default|SetbInteracted (Class|PhotonJSON|GetBoolean (Class|PhotonCloudObject|GetCustomRoomProperties (Variables|PhotonCloud|GetPhoton%20Cloud%20BP%20Ref)) (Variables|PhotonCloud|GetLeverInteractionReplicationKey)))
            (CallFunction|DOInteraction)))))))

(event EventInteract
  (params (InstigatorPawn :type Pawn%20Object%20Reference))
  ;[0.2749 0.1883 1] Local interaction
  (if (Utilities|Enum|NotEqual(Enum) (Class|SPhotonCloudObject|GetInstigatorUniqueId (Variables|PhotonCloud|GetPhoton%20Cloud%20BP%20Ref) InstigatorPawn (Variables|PhotonCloud|GetInstigator%20Unique%20Id)) "INVALID")
    (bind _returnvalue (Class|PhotonJSON|SetInteger (Class|PhotonJSON|Create self) "Instigator" (Variables|PhotonCloud|GetInstigator%20Unique%20Id)))
    (Class|PhotonCloudObject|SendObjectData (Variables|PhotonCloud|GetPhoton%20Cloud%20BP%20Ref) (Variables|PhotonCloud|GetCachedHashedName) _returnvalue 0 true "DO_NOT_CACHE" 0 "OTHERS")
    (CallFunction|ReplicateInteracted (not (Variables|Default|GetbInteracted))))
  (CallFunction|DOInteraction InstigatorPawn))

(fn ConstructionScript
  (Variables|PhotonCloud|SetCachedHashedName (Class|PhotonCloudAPIBPLibrary|GetHashedName (Utilities|GetDisplayName self))))

(fn Deserialize
  (params (data :type Photon%20JSON%20Object%20Reference))
  (return false))

(fn GetActorSeamlessTravelActorList
  (return 0))

(fn GetHashedName
  (return (Variables|PhotonCloud|GetCachedHashedName)))

(fn GetInteractDescriptionText
  (params (InstigatorPawn :type Pawn%20Object%20Reference))
  (return ""))

(fn GetInteractTitleText
  (return ""))

(fn ReceivedObjectData
  (params (data :type Photon%20JSON%20Object%20Reference))
  (Utilities|IsValid data
    (:Is%20Valid
      (bind _aspawn (Utilities|Casting|CastToPawn (Class|SPhotonCloudObject|FindInstigatorwithUniqueId (Variables|PhotonCloud|GetPhoton%20Cloud%20BP%20Ref) "PLAYER" (Class|PhotonJSON|GetInteger data "Instigator")))
        (:then
          (Variables|Default|SetbInteracted (not (Variables|Default|GetbInteracted)))
          (CallFunction|DOInteraction _aspawn)
          (return true))
        (:CastFailed
          _)))
    (:Is%20Not%20Valid
      _))
  (return false))

(fn Serialize
  (return 0))