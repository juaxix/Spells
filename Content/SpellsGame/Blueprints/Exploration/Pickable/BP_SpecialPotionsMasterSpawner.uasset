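; Spawner that places random special potions at hidden points in exploration, run only by the Photon master client in a joined room.
; On BeginPlay it runs the EQ_FindPickableSpawnPoint query in random-best-25% mode.
; On success it loops up to about SpawnCount, spawning a random PossiblePotions class at a random result via the game mode's MasterSpawnPickable.
; Each pass removes a re-randomized location, so spawn points can repeat.
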(event EventBeginPlay
  (bind _returnvalue (Subsystems|GetPhotonCloudSubsystem))
  (bind _returnvalue_2 (Class|PhotonCloudSubsystem|GetPhotonCloudAPI _returnvalue))
  (if (Utilities|Enum|Equal(Enum) (Class|PhotonCloudObject|GetState _returnvalue_2) "JOINED")
    (if (Class|PhotonCloudObject|AmIMaster _returnvalue_2)
      ;[1 1 1] find a hidden spawn to place spetial potions
      (bind _returnvalue_3 (AI|EQS|RunEQSQuery "/Game/SpellsGame/Blueprints/Exploration/Pickable/EQ_FindPickableSpawnPoint.EQ_FindPickableSpawnPoint" self "RandomBest25Pct" "/Script/AIModule.EnvQueryInstanceBlueprintWrapper"))
      (EventDispatchers|AssignOnQueryFinishedEvent _returnvalue_3 (EventDispatchers|CreateEvent :!event OnSpecialPotionsMasterSpawner)))))

(fn ConstructionScript)

(fn OnSpecialPotionsMasterSpawner
  (params (QueryInstance :type Env%20Query%20Instance%20Blueprint%20Wrapper%20Object%20Reference) (QueryStatus :type EEnvQueryStatus%20Enum :default "Processing"))
  (if (Utilities|Enum|Equal(Enum) QueryStatus "Success")
    (bind _asspells_game_mode_base (Utilities|Casting|CastToSpellsGameModeBase (Game|GetGameMode)))
    (LocalVariables|SetSpellsGameMode%20Ref _asspells_game_mode_base)
    (bind _resultlocations (AI|EQS|GetQueryResultsasLocations QueryInstance))
    (for _index (range 0 (Math|Integer|Min(Integer) (Utilities|Array|Length _resultlocations) (Variables|Spells|GetSpawnCount)))
      (Class|SpellsGameModeBase|MasterSpawnPickable (LocalVariables|GetSpellsGameMode%20Ref) (.OutItem (Utilities|Array|Random (Variables|Spells|GetPossiblePotions))) (.OutItem (Utilities|Array|Random _resultlocations)))
      (Utilities|Array|RemoveItem _resultlocations (.OutItem (Utilities|Array|Random _resultlocations))))))