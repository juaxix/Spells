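; BP_ThornsAuraPotionPickup is an exploration pickup that grants action effects, notably a thorns aura, to the character that overlaps it.
; It starts hidden without collision until a server timer fires a multicast drop that reveals it with particles and sound.
; On overlap, authority adds missing effects to damageable characters, then sets the aura's damage fraction.
; A RepNotify on the picked flag replays pickup feedback, which hides the actor before it expires.
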(event OnComponentBeginOverlap(Box)
  (params (OverlappedComponent :type Primitive%20Component%20Object%20Reference) (OtherActor :type Actor%20Object%20Reference) (OtherComp :type Primitive%20Component%20Object%20Reference) (OtherBodyIndex :type Integer) (bFromSweep :type Boolean) (SweepResult :type Hit%20Result%20Structure%20%28by%20ref%29))
  (bind _asscharacter (Utilities|Casting|CastToSCharacter OtherActor))
  (Class|SPickableInterface|Pick _asscharacter))

(event Custom|OnPicked
  (bind _returnvalue (Transformation|GetActorLocation))
  (Effects|SpawnEmitteratLocation (Variables|Default|GetPickParticleSystem) _returnvalue)
  (Audio|PlaySoundatLocation (Variables|Default|GetPickSound) _returnvalue "0, 0, 0" 0.3 1.0 0.0 0 0 0)
  (Rendering|SetActorHiddenInGame true)
  (Collision|SetCollisionEnabled (Variables|Default|GetBox) "NoCollision")
  (Actor|SetLifeSpan 3.0))

(event Custom|Multicast_Drop
  (Class|SPickableInterface|Drop (Transformation|GetActorTransform)))

(event EventBeginPlay
  (Networking|SwitchHasAuthority
    (:Authority
      (Utilities|Time|SetTimerbyEvent (delegate Custom|Multicast_Drop) (Variables|Respawn|GetTimeToShowAndEnable)))
    (:Remote
      (if (not (Variables|Default|GetbHidden))
        (Class|SPickableInterface|Drop (Transformation|GetActorTransform))))))

(event EventPick
  (params (InstigatorPawn :type Pawn%20Object%20Reference))
  (if (not (Variables|Default|GetbHidden))
    (bind _asscharacter (Utilities|Casting|CastToSCharacter InstigatorPawn))
    (if (Variables|/Script/Engine.Actor|GetbCanBeDamaged _asscharacter)
      (for _array_element (Variables|Default|GetActionEffectsGranted)
        (if (not (Class|SActionsComponent|HasAction (Variables|/Script/Spells.SCharacter|GetActionsComponent _asscharacter) _array_element))
          (Networking|SwitchHasAuthority
            (:Authority
              (Class|SActionsComponent|AddAction (Variables|/Script/Spells.SCharacter|GetActionsComponent _asscharacter) self _array_element)
              (Variables|Default|SetbPicked true)))))
      (if (Variables|Default|GetbPicked)
        (bind _assthorns_aura_action_effect (Utilities|Casting|CastToSThornsAura_ActionEffect (Class|SActionsComponent|GetAction (Variables|/Script/Spells.SCharacter|GetActionsComponent _asscharacter) "/Script/Spells.SThornsAura_ActionEffect")))
        (Variables|/Script/Spells.SThornsAura_ActionEffect|SetDamageFraction _assthorns_aura_action_effect (Variables|Default|GetThornsDamageFactor))
        (CallFunction|OnPicked)))))

(event EventDrop
  (params (DestinyTransform :type Transform%20%28by%20ref%29))
  (bind _basestaticmesh (Variables|Default|GetBaseStaticMesh))
  (Transformation|SetActorTransform DestinyTransform)
  (Rendering|SetActorHiddenInGame false)
  (Collision|SetCollisionEnabled (Variables|Default|GetBox) "QueryOnly")
  (Effects|SpawnEmitterAttached (Variables|Default|GetDropParticleSystem) _basestaticmesh "None")
  (Audio|SpawnSoundAttached (Variables|Default|GetDropSound) _basestaticmesh "None" "0, 0, 0" "0, 0, 0" "KeepRelativeOffset" false 1.0 1.0 0.0 0 0))

(fn ConstructionScript
  (Rendering|SetActorHiddenInGame true)
  (Collision|SetCollisionEnabled (Variables|Default|GetBox) "NoCollision"))

(fn OnRepBPicked
  (CallFunction|OnPicked))