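; Health potion pickup that heals an SCharacter overlapping its box, only when that character is below max health.
; It starts hidden without collision, then a timer calls Drop to reveal it with attached particles and sound.
; Pick applies the health change through the attributes component, plays effects, and hides the potion.
; If Respawn is set, Pick restarts the same timer to show it again.
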(event OnComponentBeginOverlap(Box)
  (params (OverlappedComponent :type Primitive%20Component%20Object%20Reference) (OtherActor :type Actor%20Object%20Reference) (OtherComp :type Primitive%20Component%20Object%20Reference) (OtherBodyIndex :type Integer) (bFromSweep :type Boolean) (SweepResult :type Hit%20Result%20Structure%20%28by%20ref%29))
  (bind _asscharacter (Utilities|Casting|CastToSCharacter OtherActor))
  (if (not (Variables|Default|GetbHidden))
    (Class|SPickableInterface|Pick _asscharacter)))

(event Custom|Show%20and%20Enable
  (Class|SPickableInterface|Drop (Transformation|GetActorTransform)))

(event Custom|Program%20show%20and%20enable
  (Utilities|Time|SetTimerbyEvent (delegate Custom|Show%20and%20Enable) (Variables|Default|GetTimeToShowAndEnable)))

(event EventPick
  (params (InstigatorPawn :type Pawn%20Object%20Reference))
  (bind _returnvalue (Transformation|GetActorLocation))
  (bind _self self)
  (bind _asscharacter (Utilities|Casting|CastToSCharacter InstigatorPawn))
  (if (> (Variables|/Script/Spells.SAttributesComponent|GetMaxHealth (Class|SCharacter|GetAttributesComponent _asscharacter)) (Variables|/Script/Spells.SAttributesComponent|GetHealth (Class|SCharacter|GetAttributesComponent _asscharacter)))
    (Class|SAttributesComponent|ApplyHealthChange (Class|SCharacter|GetAttributesComponent _asscharacter) (Variables|Default|GetHealth) _self (Collision|MakeHitResult false false 0.0 0.0 _returnvalue "0, 0, 0" "0,0,1" "0,0,1" 0 _self))
    (Effects|SpawnEmitteratLocation (Variables|Default|GetPickParticleSystem) _returnvalue)
    (Audio|PlaySoundatLocation (Variables|Default|GetPickSound) _returnvalue "0, 0, 0" 1.0 1.0 0.0 0 0 0)
    (Rendering|SetActorHiddenInGame true)
    (Collision|SetCollisionEnabled (Variables|Default|GetBox) "NoCollision")
    (if (Variables|Default|GetbRespawn)
      (CallFunction|ProgramShowandEnable))))

(event EventDrop
  (params (DestinyTransform :type Transform%20%28by%20ref%29))
  (bind _basestaticmesh (Variables|Default|GetBaseStaticMesh))
  (Transformation|SetActorTransform DestinyTransform)
  (Rendering|SetActorHiddenInGame false)
  (Collision|SetCollisionEnabled (Variables|Default|GetBox) "QueryOnly")
  (Effects|SpawnEmitterAttached (Variables|Default|GetDropParticleSystem) _basestaticmesh "None")
  (Audio|SpawnSoundAttached (Variables|Default|GetDropSound) _basestaticmesh "None" "0, 0, 0" "0, 0, 0" "KeepRelativeOffset" false 1.0 1.0 0.0 0 0))

(event EventBeginPlay
  (CallFunction|ProgramShowandEnable))

(fn ConstructionScript
  (Rendering|SetActorHiddenInGame true)
  (Collision|SetCollisionEnabled (Variables|Default|GetBox) "NoCollision"))