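; BP_CreditPickup is a pickup that grants credits to the player state of an SCharacter that overlaps its box.
; It starts hidden without collision, then a timer calls Drop, which reveals it, enables query collision and plays drop effects.
; Picking requires a damageable character and a positive credit value, then plays effects and hides the pickup.
; If Respawn is set, picking restarts the timer so it reappears.
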(event OnComponentBeginOverlap(Box)
  (params (OverlappedComponent :type Primitive%20Component%20Object%20Reference) (OtherActor :type Actor%20Object%20Reference) (OtherComp :type Primitive%20Component%20Object%20Reference) (OtherBodyIndex :type Integer) (bFromSweep :type Boolean) (SweepResult :type Hit%20Result%20Structure%20%28by%20ref%29))
  (bind _asscharacter (Utilities|Casting|CastToSCharacter OtherActor))
  (if (not (Variables|Default|GetbHidden))
    (Class|SPickableInterface|Pick _asscharacter)))

(event Custom|Show%20and%20Enable
  (Class|SPickableInterface|Drop (Transformation|GetActorTransform)))

(event Custom|Program%20show%20and%20enable
  (Utilities|Time|SetTimerbyEvent (delegate Custom|Show%20and%20Enable) (Variables|Respawn|GetTimeToShowAndEnable)))

(event EventPick
  (params (InstigatorPawn :type Pawn%20Object%20Reference))
  (bind _returnvalue (Transformation|GetActorLocation))
  (if (not (Variables|Default|GetbHidden))
    (bind _asscharacter (Utilities|Casting|CastToSCharacter InstigatorPawn))
    (if (and (Variables|/Script/Engine.Actor|GetbCanBeDamaged _asscharacter) (> (Variables|Default|GetCreditsGranted) 0))
      (bind _assplayer_state (Utilities|Casting|CastToSPlayerState (Variables|/Script/Engine.Pawn|GetPlayerState _asscharacter)))
      (Class|SPlayerState|GrantCredits _assplayer_state (Variables|Default|GetCreditsGranted))
      (Effects|SpawnEmitteratLocation (Variables|Default|GetPickParticleSystem) _returnvalue)
      (Audio|PlaySoundatLocation (Variables|Default|GetPickSound) _returnvalue "0, 0, 0" 0.9 1.0 0.0 "/Game/SpellsGame/Sound/SA_MagicProjectileAttenuation.SA_MagicProjectileAttenuation" 0 0)
      (Rendering|SetActorHiddenInGame true)
      (Collision|SetCollisionEnabled (Variables|Default|GetBox) "NoCollision")
      (if (Variables|Respawn|GetbRespawn)
        (CallFunction|ProgramShowandEnable)))))

(event EventDrop
  (params (DestinyTransform :type Transform%20%28by%20ref%29))
  (bind _basestaticmesh (Variables|Default|GetBaseStaticMesh))
  (Transformation|SetActorTransform DestinyTransform)
  (Rendering|SetActorHiddenInGame false)
  (Collision|SetCollisionEnabled (Variables|Default|GetBox) "QueryOnly")
  (Effects|SpawnEmitterAttached (Variables|Default|GetDropParticleSystem) _basestaticmesh "None")
  (Audio|SpawnSoundAttached (Variables|Default|GetDropSound) _basestaticmesh "None" "0, 0, 0" "0, 0, 0" "KeepRelativeOffset" false 1.0 1.0 0.0 0 0))

(event EventBeginPlay
  (CallFunction|ProgramShowandEnable))

(fn ConstructionScript
  (Rendering|SetActorHiddenInGame true)
  (Collision|SetCollisionEnabled (Variables|Default|GetBox) "NoCollision"))