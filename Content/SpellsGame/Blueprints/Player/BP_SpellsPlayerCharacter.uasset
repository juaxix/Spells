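; Player character Blueprint for a spell-casting game, handling HUD setup, damage feedback and the character's starting actions.
; The construction script registers sprint, magic projectile, teleport and black hole actions with the ActionsComponent.
; BeginPlay adds crosshair and game display widgets and starts a camera shake; unpossession removes both widgets.
; Health loss reported by the AttributesComponent writes game time to the mesh materials' TimeToHit parameter.
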(event OnHealthAttributeChanged(AttributesComponent)
  (params (InstigatorActor :type Actor%20Object%20Reference) (AttributeComponent :type S%20Attributes%20Component%20Object%20Reference) (NewHealth :type Float%20%28single-precision%29) (Delta :type Float%20%28single-precision%29) (Hit :type Hit%20Result%20Structure%20%28by%20ref%29))
  (if (< Delta 0.0)
    (Rendering|Material|SetScalarParameterValueonMaterials (Variables|Character|GetMesh) "TimeToHit" (Utilities|Time|GetGameTimeinSeconds))))

(event EventBeginPlay
  (bind _returnvalue (Pawn|GetController))
  (bind _asplayer_controller (Utilities|Casting|CastToPlayerController _returnvalue))
  (bind _returnvalue_2 (UserInterface|CreateWidget "/Game/SpellsGame/UI/Player/Widget_Crosshair.Widget_Crosshair_C" _asplayer_controller))
  (bind _output_get (Variables|Default|SetWBP_Crossair _returnvalue_2))
  (UserInterface|Viewport|AddtoViewport _output_get 0)
  (bind _returnvalue_3 (UserInterface|CreateWidget "/Game/SpellsGame/UI/Player/Widget_GameDisplay.Widget_GameDisplay_C" _asplayer_controller))
  (bind _output_get_2 (Variables|Default|SetWBP_PlayerAttributes _returnvalue_3))
  (UserInterface|Viewport|AddtoViewport _output_get_2 0)
  (Class|MatineeCameraShake|StartMatineeCameraShake 0 "/Script/GameplayCameras.MatineeCameraShake" 1.0 "CameraLocal" "0, 0, 0"))

(event EventUnpossessed
  (params (OldController :type Controller%20Object%20Reference))
  (Widget|RemovefromParent (Variables|Default|GetWBP_Crossair)))

(fn ConstructionScript
  (bind _actionscomponent (Variables|Default|GetActionsComponent))
  (Class|SActionsComponent|AddAction _actionscomponent "/Game/SpellsGame/Blueprints/Gameplay/Actions/BP_SprintAction.BP_SprintAction_C")
  (Class|SActionsComponent|AddAction _actionscomponent "/Game/SpellsGame/Blueprints/Gameplay/Actions/BP_MagicProjectileAttack_Action.BP_MagicProjectileAttack_Action_C")
  (Class|SActionsComponent|AddAction _actionscomponent "/Game/SpellsGame/Blueprints/Gameplay/Actions/BP_Teleport_Action.BP_Teleport_Action_C")
  (Class|SActionsComponent|AddAction _actionscomponent "/Game/SpellsGame/Blueprints/Gameplay/Actions/BP_Blackhole_Action.BP_Blackhole_Action_C"))