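; BP_AttackTower is an enemy tower that turns toward a character and fires magic projectiles at it.
; BeginPlay caches the first SCharacter found as NearestCharacter, with no distance check or later update, and starts a looping three-second timer.
; Each timer firing spawns a BP_SpellsMagicProjectile from the tower's location, aimed straight at the target regardless of tower facing.
; Tick eases the tower's rotation toward the target using a DeltaSeconds lerp.
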(event Custom|Shoot%20Nearest%20Player%20Char
  (bind _returnvalue (Transformation|GetActorLocation))
  (Game|SpawnActorfromClass "/Game/SpellsGame/Blueprints/Attacks/BP_SpellsMagicProjectile.BP_SpellsMagicProjectile_C" (Math|Transform|MakeTransform _returnvalue (Math|Rotator|MakeRotfromX (- (Transformation|GetActorLocation (Variables|Default|GetNearestCharacter)) _returnvalue)) "1,1,1") "Undefined" self 0))

(event EventTick
  (params (DeltaSeconds :type Float%20%28single-precision%29))
  (Transformation|SetActorRotation (Math|Rotator|Lerp(Rotator) (Transformation|GetActorRotation) (Math|Rotator|MakeRotfromX (- (Transformation|GetActorLocation (Variables|Default|GetNearestCharacter)) (Transformation|GetActorLocation))) DeltaSeconds)))

(event EventBeginPlay
  (Utilities|Time|SetTimerbyEvent (delegate Custom|Shoot%20Nearest%20Player%20Char) 3.0 true 1.0)
  (bind _outactors (Actor|GetAllActorsOfClass "/Script/Spells.SCharacter"))
  (Variables|Default|SetNearestCharacter (Utilities|Array|Get(acopy) _outactors)))

(fn ConstructionScript)