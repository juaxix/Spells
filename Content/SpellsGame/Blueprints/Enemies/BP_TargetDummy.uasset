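; BP_TargetDummy is an enemy target dummy that shows a running total of health changes in an on-screen damage counter.
; On each health attribute change it creates or reuses a single counter widget attached to itself and re-adds it to the viewport if needed.
; It adds the delta to the number parsed from the widget's text, then resets the widget's lifespan and offset.
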(event OnHealthAttributeChanged(AttributesComponent)
  (params (InstigatorActor :type Actor%20Object%20Reference) (AttributeComponent :type S%20Attributes%20Component%20Object%20Reference) (NewValue :type Float%20%28single-precision%29) (Delta :type Float%20%28single-precision%29) (Hit :type Hit%20Result%20Structure%20%28by%20ref%29))
  (Variables|Default|GetDamageCounter
    (:then
      _)
    (:else
      (bind _returnvalue (UserInterface|CreateWidget "/Game/SpellsGame/Blueprints/Widgets/Widget_DamageCounter.Widget_DamageCounter_C" 0 self))
      (Variables|Default|SetDamageCounter _returnvalue)))
  (if (UserInterface|Viewport|IsinViewport (Variables|Default|GetDamageCounter))
    _
    (else
      (UserInterface|Viewport|AddtoViewport (Variables|Default|GetDamageCounter) 0)))
  (Variables|/Game/SpellsGame/Blueprints/Widgets/Widget_DamageCounter.Widget_DamageCounter_C|SetLifespan (Variables|Default|GetDamageCounter) 2.2)
  (Rendering|Components|TextRender|SetText (Variables|/Game/SpellsGame/Blueprints/Widgets/Widget_DamageCounter.Widget_DamageCounter_C|GetText_Damage (Variables|Default|GetDamageCounter)) (Utilities|Text|ToText(Float) (+ Delta (Math|Conversions|ToFloat(Integer) (Utilities|String|ToString(Text) (Class|TextBlock|GetText (Variables|/Game/SpellsGame/Blueprints/Widgets/Widget_DamageCounter.Widget_DamageCounter_C|GetText_Damage (Variables|Default|GetDamageCounter)))))) "HalfToEven"))
  (Variables|/Game/SpellsGame/Blueprints/Widgets/Widget_DamageCounter.Widget_DamageCounter_C|SetOffset (Variables|Default|GetDamageCounter) "0, 0, 0"))

(fn ConstructionScript)