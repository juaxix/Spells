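; EQS query context that supplies all player characters as an actor set for enemy AI environment queries.
; It walks the GameState's PlayerArray and keeps each pawn whose class is SCharacter or a child of it.
; Without a valid GameState it falls back to GetAllActorsOfClass on SCharacter, a costlier path noted as editor-only.
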(fn ProvideActorsSet
  (params (QuerierObject :type Object%20Object%20Reference) (QuerierActor :type Actor%20Object%20Reference))
  (bind _returnvalue (Game|GetGameState))
  (Utilities|IsValid _returnvalue
    (:Is%20Valid
      (for _array_element (Variables|/Script/Engine.GameStateBase|GetPlayerArray _returnvalue)
        (if (or (== (Utilities|GetClass (Variables|/Script/Engine.PlayerState|GetPawnPrivate _array_element)) "/Script/Spells.SCharacter") (Utilities|ClassIsChildOf (Utilities|GetClass (Variables|/Script/Engine.PlayerState|GetPawnPrivate _array_element)) "/Script/Spells.SCharacter"))
          (Utilities|Array|Add (LocalVariables|GetPlayerActors) (Variables|/Script/Engine.PlayerState|GetPawnPrivate _array_element))))
      (return (LocalVariables|GetPlayerActors)))
    (:Is%20Not%20Valid
      ;[1 1 1] cache if it's expensive - Only for editor though
      (bind _outactors (Actor|GetAllActorsOfClass "/Script/Spells.SCharacter"))
      (return _outactors))))