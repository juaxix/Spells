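; BP_PhotonCloudObject is a Photon Cloud connection object for online play that logs connection activity to the screen.
; On initialization it calls the parent, prints a startup message and binds handlers for the cloud state-changed and connection-error events.
; Those handlers print each new state name and any error message.
; A disconnect timeout call is present but unconnected, so it never runs.
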(event Custom|On%20Photon%20Cloud%20State%20Changed
  (params (NewState :type EPhotonCloudStates%20Enum :default "UNINITIALIZED"))
  (Development|PrintString self (Utilities|String|Append "Photon Cloud State: " (Utilities|String|EnumtoString NewState))))

(event Custom|On%20Photon%20Connection%20Error
  (params (ErrorCode :type EPhotonErrorCode%20Enum :default "OK") (ErrorMessage :type String))
  (Development|PrintString self ErrorMessage))

(event EventOnPhotonCloudInitialized
  (|CallParentFunction)
  (Development|PrintString self "Photon Cloud Object init")
  (EventDispatchers|AssignOnPhotonCloudStateChanged (delegate Custom|On%20Photon%20Cloud%20State%20Changed))
  (EventDispatchers|AssignOnPhotonConnectionError (delegate Custom|On%20Photon%20Connection%20Error)))