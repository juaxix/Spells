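; BP_Blackhole_Action is the Blackhole spell action, gated by and paid for with the caster's Rage.
; CanStart adds a Rage check to the parent's conditions and prints a message when Rage is short of RageCost.
; StartAction runs the parent action for a valid instigator, then deducts RageCost through the attributes component's ApplyRageChange.
; The black hole behavior itself is left to the parent class.
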(event EventStartAction
  (params (Instigator :type Actor%20Object%20Reference))
  (Utilities|IsValid Instigator
    (:Is%20Valid
      (|CallParentFunction Instigator)
      (Class|SAttributesComponent|ApplyRageChange (Class|SAttributesComponent|GetAttributesComponent Instigator) (* (Variables|Default|GetRageCost) -1.0) Instigator (Collision|MakeHitResult false false 0.0 0.0 (Transformation|GetActorLocation Instigator) "0, 0, 0" "0,0,1" "0,0,1" 0 0)))))

(fn CanStart
  (params (Instigator :type Actor%20Object%20Reference))
  (if (|CallParentFunction Instigator)
    (bind _output_get (LocalVariables|SetAttributes (Class|SAttributesComponent|GetAttributesComponent Instigator)))
    (Utilities|IsValid _output_get
      (:Is%20Valid
        (if (>= (Variables|/Script/Spells.SAttributesComponent|GetRage (LocalVariables|GetAttributes)) (Variables|Default|GetRageCost))
          (return true)
          (else
            (Development|PrintString 0 "Not enough Rage to cast this spell")
            (return false))))
      (:Is%20Not%20Valid
        _)))
  (return false))