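; BP_Teleport_Action is the teleport spell action, adding a mana cost on top of its parent action.
; CanStart requires the parent check to pass and the instigator's attributes component to hold enough Mana, printing a message when it falls short.
; StartAction runs the parent's start logic, then deducts ManaCost through ApplyManaChange.
; The teleport itself is not implemented in these graphs.
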(event EventStartAction
  (params (Instigator :type Actor%20Object%20Reference))
  (bind _returnvalue (Transformation|GetActorLocation Instigator))
  (bind _returnvalue_2 (Class|SAttributesComponent|GetAttributesComponent Instigator))
  (|CallParentFunction Instigator)
  (Utilities|IsValid _returnvalue_2
    (:Is%20Valid
      (Class|SAttributesComponent|ApplyManaChange _returnvalue_2 (* (Variables|Default|GetManaCost) -1.0) Instigator (Collision|MakeHitResult false false 0.0 0.0 _returnvalue _returnvalue "0,0,1" "0,0,1" 0 0)))))

(fn CanStart
  (params (Instigator :type Actor%20Object%20Reference))
  (if (|CallParentFunction Instigator)
    (if (>= (Variables|/Script/Spells.SAttributesComponent|GetMana (Class|SAttributesComponent|GetAttributesComponent Instigator)) (Variables|Default|GetManaCost))
      (return true)
      (else
        (Development|PrintString 0 "Not enough Mana to cast this spell")
        (return false)))
    (else
      (return false))))