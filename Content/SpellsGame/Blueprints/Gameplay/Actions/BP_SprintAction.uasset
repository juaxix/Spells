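; Sprint action Blueprint that temporarily raises a character's walk speed while active.
; On start, it calls the parent logic, casts the instigator to Character and adds BonusSpeed to the movement component's MaxWalkSpeed.
; On stop, it calls the parent logic and subtracts the same variable, an additive change rather than restoring a cached value.
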(event EventStartAction
  (params (Instigator :type Actor%20Object%20Reference))
  (|CallParentFunction Instigator)
  (bind _ascharacter (Utilities|Casting|CastToCharacter Instigator))
  (Variables|/Script/Engine.CharacterMovementComponent|SetMaxWalkSpeed (Variables|/Script/Engine.Character|GetCharacterMovement _ascharacter) (+ (Variables|/Script/Engine.CharacterMovementComponent|GetMaxWalkSpeed (Variables|/Script/Engine.Character|GetCharacterMovement _ascharacter)) (Variables|Default|GetBonusSpeed))))

(event EventStopAction
  (params (Instigator :type Actor%20Object%20Reference))
  (|CallParentFunction Instigator)
  (bind _ascharacter (Utilities|Casting|CastToCharacter Instigator))
  (Variables|/Script/Engine.CharacterMovementComponent|SetMaxWalkSpeed (Variables|/Script/Engine.Character|GetCharacterMovement _ascharacter) (- (Variables|/Script/Engine.CharacterMovementComponent|GetMaxWalkSpeed (Variables|/Script/Engine.Character|GetCharacterMovement _ascharacter)) (Variables|Default|GetBonusSpeed))))